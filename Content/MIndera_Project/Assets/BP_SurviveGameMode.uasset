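; BP_SurviveGameMode is the game mode for the survive mode, scoring the player for time survived.
; On BeginPlay it looks up the current character in the project instance, applies it to the first-person character and shows WBP_SurviveUI.
; AddScore re-calls itself through a Gate and one-second Delay to increment the score.
; EndGame closes that Gate, toggles the widget's end-game visibility and, after a short delay, opens LV_MainLevel.
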(event Custom|Add%20Score
  (Utilities|FlowControl|Gate false
    (:Exit
      (Math|Integer|IncrementInt (Variables|Default|GetiGameScore)
        (:%20%20
          (Utilities|FlowControl|Delay 1.0)
          (CallFunction|AddScore))))))

(event EventBeginPlay
  (bind (_cast_ _asbp_first_person_character) (CallFunction|GetProjectCharacter))
  (bind (_output _character_found) (Default|IBPGetCharacterbyInt (CallFunction|GetProjectInstance) (Variables|Default|GetiCurrentCharacter)))
  (if _character_found
    (if _cast_
      (Default|ChangeCharacter _asbp_first_person_character _output)
      (bind _returnvalue (UserInterface|CreateWidget "/Game/MIndera_Project/Assets/Widgets/WBP_SurviveUI.WBP_SurviveUI_C" (Game|GetPlayerController 0)))
      (bind _output_get (Variables|Default|SetwbpSurviveWidget _returnvalue))
      (UserInterface|Viewport|AddtoViewport _output_get 0)
      (CallFunction|AddScore))))

(event EventTick
  (params (DeltaSeconds :type Float%20%28single-precision%29)))

(event EventEndGame
  (Utilities|FlowControl|Sequence
    (:then_0
      (Utilities|FlowControl|Gate false) ; enters at Close
    )
    (:then_1
      (Default|EndGameVisibilityChange (Variables|Default|GetwbpSurviveWidget))
      (Utilities|FlowControl|Delay 2.0)
      (Game|OpenLevel(byName) "LV_MainLevel"))))

(fn ConstructionScript)